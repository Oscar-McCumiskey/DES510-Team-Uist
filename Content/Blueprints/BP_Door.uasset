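; BP_Door is a door that swings open and closed around its yaw axis.
; Box overlap begin and end play separate open and close timelines from the start, each driving the Door's relative rotation.
; An Interact event flips a boolean to alternate between the same two paths, re-entering at their BP_ThirdPersonCharacter casts, which still read the overlap events' OtherActor.
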(event `self.Box.OnComponentBeginOverlap`
  (params (OverlappedComponent :type "PrimitiveComponent Object Reference") (OtherActor :type "Actor Object Reference") (OtherComp :type "PrimitiveComponent Object Reference") (OtherBodyIndex :type Integer) (bFromSweep :type Boolean) (SweepResult :type "HitResult Structure (by ref)"))
  (cast `/Game/ThirdPerson/Blueprints/BP_ThirdPersonCharacter` OtherActor :!label _label)
  (bind (_direction _rotationrate) (`Timeline|TimelineOpenDoor` :!via `PlayFromStart`)
    (:`Update`
      (`SceneComponent.K2_SetRelativeRotation` (`self.Door`) (`KismetMathLibrary.MakeRotator` 0.0 0.0 _rotationrate) false false))))

(event `self.Box.OnComponentEndOverlap`
  (params (OverlappedComponent :type "PrimitiveComponent Object Reference") (OtherActor :type "Actor Object Reference") (OtherComp :type "PrimitiveComponent Object Reference") (OtherBodyIndex :type Integer))
  (cast `/Game/ThirdPerson/Blueprints/BP_ThirdPersonCharacter` OtherActor :!label _label_2)
  (bind (_direction _rotationrate) (`Timeline|TimelineDoorClose` :!via `PlayFromStart`)
    (:`Update`
      (`SceneComponent.K2_SetRelativeRotation` (`self.Door`) (`KismetMathLibrary.MakeRotator` 0.0 0.0 _rotationrate) false false))))

(event `/Game/Blueprints/Interfaces/BPI_Interact.Interact`
  (bind _condition (`self.Condition`))
  (set `self.Condition` (not _condition))
  (if _condition
    (goto _label)
    (else
      (goto _label_2))))

(fn `UserConstructionScript`)