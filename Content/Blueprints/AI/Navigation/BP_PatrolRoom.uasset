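; BP_PatrolRoom represents one room on an AI patrol route and hands out waypoint locations within it.
; On BeginPlay it gathers the capsule locations of every BP_Waypoint with a matching RoomID into a shuffled list.
; GetNextWaypoint returns the current entry and advances a wrapping index, signalling a room change and reshuffling when the index returns to zero or the Spooked input is set.
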(event `self.ReceiveBeginPlay`
  (bind _waypoints (`self.Waypoints`))
  (bind _outactors (`GameplayStatics.GetAllActorsOfClass` "/Game/Blueprints/AI/Navigation/BP_Waypoint.BP_Waypoint_C"))
  (for _array_element _outactors
    (if (`|EnumEquality` (`/Game/Blueprints/AI/Navigation/BP_Waypoint.RoomID` _array_element) (`self.RoomID`))
      (`KismetArrayLibrary.Array_Add` _waypoints (`SceneComponent.K2_GetComponentLocation` (`/Game/Blueprints/AI/Navigation/BP_Waypoint.Capsule` _array_element)))
      (`KismetArrayLibrary.Array_Shuffle` _waypoints))))

(fn `GetNextWaypoint`
  (params (Spooked :type Boolean))
  (returns (ChangeRoom :type Boolean) (Waypoint :type "Vector Structure"))
  (bind _selectedwaypoint (`self.SelectedWaypoint`))
  (set `self.SelectedWaypoint` (`|GetArrayItem` (`self.Waypoints`) (`self.WaypointIndex`)))
  (bind _output_get (set `self.WaypointIndex` (`KismetMathLibrary.Wrap` (+ (`self.WaypointIndex`) 1) -1 (- (`KismetArrayLibrary.Array_Length` (`self.Waypoints`)) 1))))
  (if (or Spooked (== _output_get 0))
    (set `self.WaypointIndex` 0)
    (`KismetArrayLibrary.Array_Shuffle` (`self.Waypoints`))
    (return true _selectedwaypoint)
    (else
      (return false _selectedwaypoint))))

(fn `UserConstructionScript`)