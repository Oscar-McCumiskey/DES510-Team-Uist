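; BP_RobotButler is the robot butler actor, with a widget component that shows a state icon.
; On BeginPlay it caches the W_StateIcon widget, hides it and posts the Wwise robot movement event on itself.
; DisplayStateIcon sets the widget's image and makes it visible without hit testing on itself, and HideStateIcon hides it through the cached reference.
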(event `self.ReceiveBeginPlay`
  (bind _asw_state_icon (cast `/Game/Blueprints/AI/State_Icons/W_StateIcon` (`WidgetComponent.GetWidget` (`self.StateIcon`))))
  (set `self.StateIconWidget` _asw_state_icon)
  (`self.HideStateIcon`)
  (`AkGameplayStatics.PostEvent` "/Game/WwiseAudio/Events/Default_Work_Unit/AkEvent_RobotMovement.AkEvent_RobotMovement" self))

(fn `DisplayStateIcon`
  (params (StateIcon :type "/Game/Blueprints/Enumerators/E_RobotButlerState Enum" :default "NewEnumerator0"))
  (bind _asw_state_icon (cast `/Game/Blueprints/AI/State_Icons/W_StateIcon` (`WidgetComponent.GetWidget` (`self.StateIcon`))))
  (`/Game/Blueprints/AI/State_Icons/W_StateIcon.SetImage` _asw_state_icon StateIcon)
  (`Widget.SetVisibility` _asw_state_icon "HitTestInvisible"))

(fn `HideStateIcon`
  (`Widget.SetVisibility` (`self.StateIconWidget`) "Hidden"))

(fn `UserConstructionScript`)