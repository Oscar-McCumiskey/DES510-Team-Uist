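; AI controller for the robot butler, which patrols shuffled rooms, hunts the unpossessed player and can be scared by tagged noises.
; Perception feeds a StateTree: nearby, unobstructed noises trigger tagged reactions and add multiplied shock to the player controller, while sight starts detection.
; Tick checks range and line of sight, drives detection UI and reports detection once.
; When shock maxes out, it stops and hides the robot.
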(event `self.ReceiveBeginPlay`
  (bind _patrolrooms (`self.PatrolRooms`))
  (`|ExecutionSequence`
    (:`then_0`
      ;[0 0.875 0.1167 0.5 30] Patrol State
      (bind _outactors (`GameplayStatics.GetAllActorsOfClass` "/Game/Blueprints/AI/Navigation/BP_PatrolRoom.BP_PatrolRoom_C"))
      (for _array_element _outactors
        (if (`/Game/Blueprints/AI/Navigation/BP_PatrolRoom.IsActive` _array_element)
          (`KismetArrayLibrary.Array_Add` _patrolrooms _array_element)
          (`KismetArrayLibrary.Array_Shuffle` _patrolrooms)
          (set `self.CurrentPatrolRoom` (`|GetArrayItem` _patrolrooms))
          (bind _outactors_2 (`GameplayStatics.GetAllActorsOfClass` "/Script/DES510_Team_Uist.PossessableAppliance"))
          (bind _output_get (set `self.IgnoreActors` _outactors_2))
          (`KismetArrayLibrary.Array_Add` _output_get (`self.K2_GetPawn`))))
      (set `self.RoomIndex` 0))
    (:`then_2`
      ; Start State Tree
      (`BrainComponent.StartLogic` (`self.StateTreeAI`)))
    (:`then_3`
      (bind _asbp_third_person_player_controller (cast `/Game/ThirdPerson/Blueprints/BP_ThirdPersonPlayerController` (`GameplayStatics.GetPlayerController` 0)))
      (set `self.PlayerController` _asbp_third_person_player_controller))))

(event `self.AIPerception.OnTargetPerceptionUpdated`
  (params (Actor :type "Actor Object Reference") (Stimulus :type "AIStimulus Structure"))
  (bind (_age _expirationage _strength _stimuluslocation _receiverlocation _tag _bsuccessfullysensed) (break `AIStimulus` Stimulus))
  (bind _sensetype (`self.GetSenseType` Stimulus))
  (switch `/Game/Blueprints/Enumerators/E_SenseType` _sensetype
    (:`NewEnumerator1`
      ;[0.9479 0.9101 0.02885 0.5 32] Hearing States
      (if (and (not (`self.IsSpooked`)) _bsuccessfullysensed)
        (bind _output_get (set `self.LastStimulusLocation` _stimuluslocation))
        (bind (_outhit _returnvalue) (`KismetSystemLibrary.LineTraceSingle` (`self.K2_GetActorLocation` (`self.K2_GetPawn`)) _output_get "TraceTypeQuery1" false (`self.IgnoreActors`) "ForDuration"))
        (if (and (< (`KismetMathLibrary.Vector_Distance` _output_get (`self.K2_GetActorLocation` (`self.K2_GetPawn`))) (`self.ScareDistance`)) (not _returnvalue))
          (switch `name` _tag
            (:`Default`
              (`self.RobotSoundEvent` "/Game/WwiseAudio/Events/Default_Work_Unit/AkEvent_RobotAlert.AkEvent_RobotAlert" (struct :`TagName` "StateTree.Scared") true 4.0 "NewEnumerator2"))
            (:`AlertVisual`
              (`self.RobotSoundEvent` "/Game/WwiseAudio/Events/Default_Work_Unit/AkEvent_RobotAlert.AkEvent_RobotAlert" (struct :`TagName` "StateTree.Scared") true 4.0 "NewEnumerator0"))
            (:`AlertAudio`
              (`self.RobotSoundEvent` "/Game/WwiseAudio/Events/Default_Work_Unit/AkEvent_RobotAlert.AkEvent_RobotAlert" (struct :`TagName` "StateTree.Scared") true 4.0))
            (:`PanicVisual`
              (`self.RobotSoundEvent` "/Game/WwiseAudio/Events/Default_Work_Unit/AkEvent_RobotAlert.AkEvent_RobotAlert" (struct :`TagName` "StateTree.Panic") true 6.0 "NewEnumerator0"))
            (:`PanicAudio`
              (`self.RobotSoundEvent` "/Game/WwiseAudio/Events/Default_Work_Unit/AkEvent_RobotAlert.AkEvent_RobotAlert" (struct :`TagName` "StateTree.Panic") true 6.0))
            (:`DanceVisual`
              (`self.RobotSoundEvent` "/Game/WwiseAudio/Events/Default_Work_Unit/AkEvent_RobotAlert.AkEvent_RobotAlert" (struct :`TagName` "StateTree.Dance") true 6.0 "NewEnumerator0"))
            (:`DanceAudio`
              (`self.RobotSoundEvent` "/Game/WwiseAudio/Events/Default_Work_Unit/AkEvent_RobotAlert.AkEvent_RobotAlert" (struct :`TagName` "StateTree.Dance") true 6.0))
            (:`SpookedVisual`
              (set `self.IsSpooked` true)
              (set `self.RoomChangeOverride` true)
              (`self.RobotSoundEvent` "/Game/WwiseAudio/Events/Default_Work_Unit/AkEvent_RobotAlert.AkEvent_RobotAlert" (struct :`TagName` "StateTree.Spooked") true 4.0 "NewEnumerator0"))
            (:`SpookedAudio`
              (set `self.IsSpooked` true)
              (set `self.RoomChangeOverride` true)
              (`self.RobotSoundEvent` "/Game/WwiseAudio/Events/Default_Work_Unit/AkEvent_RobotAlert.AkEvent_RobotAlert" (struct :`TagName` "StateTree.Spooked") true 4.0))
            (:`Debug`
              (`self.RobotSoundEvent` "/Game/WwiseAudio/Events/Default_Work_Unit/AkEvent_RobotAlert.AkEvent_RobotAlert" (struct :`TagName` "StateTree.Debug") true 5.0 "NewEnumerator2")))
          (elif (!= _tag "Search")
            _))))
    (:`NewEnumerator0`
      ;[0.9479 0.1913 0 0.5 32] Sight States
      (if (`.bSuccessfullySensed` (break `AIStimulus` Stimulus))
        (if (and (== (`GameplayStatics.GetObjectClass` Actor) "/Game/ThirdPerson/Blueprints/BP_ThirdPersonCharacter.BP_ThirdPersonCharacter_C") (not (`/Game/ThirdPerson/Blueprints/BP_ThirdPersonPlayerController.PossessingAppliance` (`self.PlayerController`))))
          (set `self.TargetPlayer` Actor)
          (set `self.SeeingPlayer` true)
          (if (not (`self.Detected`))
            (`StateTreeComponent.SendStateTreeEvent` (`self.StateTreeAI`) (make `StateTreeEvent` (struct :`TagName` "StateTree.Detected")))))))
    (:`NewEnumerator2`
      (`KismetSystemLibrary.PrintString` "Unknown Sense"))))

(event `self.AIPerception.OnTargetPerceptionForgotten`
  (params (Actor :type "Actor Object Reference"))
  ;[0.9479 0.1913 0 0.5 32] Sight States
  (if (== Actor (`self.TargetPlayer`))
    (set `self.SeeingPlayer` false)))

(event `self.ReceiveTick`
  (params (DeltaSeconds :type "Float (single-precision)"))
  (bind _returnvalue (`self.K2_GetPawn`))
  (bind _playercontroller (`self.PlayerController`))
  (bind _targetplayer (`self.TargetPlayer`))
  (bind _returnvalue_2 (`self.K2_GetActorLocation` (`self.K2_GetPawn`)))
  (bind _returnvalue_3 (`self.K2_GetActorLocation` _targetplayer))
  (bind _returnvalue_4 (+ (`self.OutOfLOSTimer`) DeltaSeconds))
  ;[0.9479 0.1913 0 0.5 32] Sight States
  (`|ExecutionSequence`
    (:`then_0`
      (`/Engine/EditorBlueprintResources/StandardMacros.IsValid` _targetplayer
        (:`Is Valid`
          (bind _output_get (set `self.Distance` (`KismetMathLibrary.Vector_Distance` _returnvalue_2 _returnvalue_3)))
          (if (or (>= _output_get 1000.0) (`/Game/ThirdPerson/Blueprints/BP_ThirdPersonPlayerController.PossessingAppliance` (`self.PlayerController`)))
            (set `self.SeeingPlayer` false)
            (set `self.OutOfLOSTimer` 0.0)
            (else
              (bind (_outhit _returnvalue_5) (`KismetSystemLibrary.LineTraceSingle` _returnvalue_2 _returnvalue_3 "TraceTypeQuery2" false (`|MakeArray` (`self.TargetPlayer`) (`self.K2_GetPawn`) :!type "Actor Object Reference")))
              (if _returnvalue_5
                (set `self.OutOfLOSTimer` _returnvalue_4)
                (if (>= _returnvalue_4 0.2)
                  (set `self.SeeingPlayer` false)
                  (set `self.OutOfLOSTimer` 0.0))
                (else
                  (set `self.OutOfLOSTimer` 0.0))))))))
    (:`then_1`
      (if (`self.Detected`)
        (if (not (`self.DeathConsumed`))
          (set `self.DeathConsumed` true)
          (`/Game/ThirdPerson/Blueprints/BP_ThirdPersonPlayerController.PlayerDetected` (`self.PlayerController`))
          (`/Game/ThirdPerson/Blueprints/BP_ThirdPersonPlayerController.UpdateDetectionUI` (`self.PlayerController`) 100.0 true "HitTestInvisible"))
        (elif (`self.SeeingPlayer`)
          (`/Game/ThirdPerson/Blueprints/BP_ThirdPersonPlayerController.UpdateDetectionUI` (`self.PlayerController`) (`self.DetectionProgress`) false "HitTestInvisible")
          (elif (<= (`self.DetectionProgress`) 0.0)
            (`/Game/ThirdPerson/Blueprints/BP_ThirdPersonPlayerController.UpdateDetectionUI` (`self.PlayerController`) (`self.DetectionProgress`) false "Hidden")
            (else
              (`/Game/ThirdPerson/Blueprints/BP_ThirdPersonPlayerController.UpdateDetectionUI` (`self.PlayerController`) (`self.DetectionProgress`) false "HitTestInvisible"))))))
    (:`then_2`
      (if (>= (`DES510_Team_UistPlayerController.CurrentShock` _playercontroller) (`DES510_Team_UistPlayerController.MaxShock` _playercontroller))
        (`MovementComponent.StopMovementImmediately` (`Pawn.GetMovementComponent` _returnvalue))
        (`BrainComponent.StopLogic` (`self.StateTreeAI`) "")
        (`self.SetActorHiddenInGame` _returnvalue true)))))

(fn `ChangeSpookCount`
  (params (Value :type Integer))
  (returns (SpookCount :type Integer))
  (bind _output_get (set `self.SpookCount` (+ Value (`self.SpookCount`))))
  (return _output_get))

(fn `GenerateShock`
  (params (ShockGenerated :type "Float (double-precision)") (SenseType :type "/Game/Blueprints/Enumerators/E_SenseType Enum" :default "NewEnumerator1"))
  (bind _asbp_third_person_player_controller (cast `/Game/ThirdPerson/Blueprints/BP_ThirdPersonPlayerController` (`GameplayStatics.GetPlayerController` 0)))
  (`/Game/ThirdPerson/Blueprints/BP_ThirdPersonPlayerController.SetMultiplierTimer` _asbp_third_person_player_controller SenseType (`self.MultiplierDuration`))
  (bind _multiplier (`/Game/ThirdPerson/Blueprints/BP_ThirdPersonPlayerController.GetShockMultiplier` _asbp_third_person_player_controller))
  (`DES510_Team_UistPlayerController.AddShock` _asbp_third_person_player_controller (* _multiplier ShockGenerated))
  (`KismetSystemLibrary.PrintString` (`KismetStringLibrary.Concat_StrStr` "Multiplier: " (`KismetStringLibrary.Conv_DoubleToString` _multiplier))))

(fn `GetNextPatrolPoint`
  (params (Spooked :type Boolean))
  (returns (PatrolPoint :type "Vector Structure"))
  (if Spooked
    (bind _output_get (set `self.RoomIndex` (`KismetMathLibrary.Wrap` (+ (`self.RoomIndex`) 1) -1 (- (`KismetArrayLibrary.Array_Length` (`self.PatrolRooms`)) 1)))))
  (bind (_changeroom _waypoint) (`/Game/Blueprints/AI/Navigation/BP_PatrolRoom.GetNextWaypoint` (`|GetArrayItem` (`self.PatrolRooms`) _output_get) Spooked))
  (if (or (`self.RoomChangeOverride`) _changeroom)
    (set `self.RoomChangeOverride` false)
    (bind _output_get_2 (set `self.RoomIndex` (`KismetMathLibrary.Wrap` (+ (`self.RoomIndex`) 1) -1 (- (`KismetArrayLibrary.Array_Length` (`self.PatrolRooms`)) 1))))
    (if (== _output_get_2 0)
      _
      (else
        _))
    (return _waypoint)
    (else
      (return _waypoint))))

(fn `GetNextPatrolRoom`
  (returns (PatrolRoom :type "Vector Structure"))
  (bind _output_get (set `self.RoomIndex` (`KismetMathLibrary.Wrap` (+ (`self.RoomIndex`) 1) -1 (- (`KismetArrayLibrary.Array_Length` (`self.PatrolRooms`)) 1))))
  (bind _output_get_2 (set `self.CurrentPatrolRoom` (`|GetArrayItem` (`self.PatrolRooms`) _output_get)))
  (return (`self.K2_GetActorLocation` _output_get_2)))

(fn `GetNextWaypoint`
  (returns (ChangeRoom :type Boolean) (Location :type "Vector Structure"))
  (bind (_changeroom _waypoint) (`/Game/Blueprints/AI/Navigation/BP_PatrolRoom.GetNextWaypoint` (`self.CurrentPatrolRoom`) false))
  (return _changeroom _waypoint))

(fn `GetSenseType`
  (params (Stimuli :type "AIStimulus Structure"))
  (returns (SenseType :type "/Game/Blueprints/Enumerators/E_SenseType Enum"))
  (bind _returnvalue (`AIPerceptionSystem.GetSenseClassForStimulus` Stimuli))
  (if (== _returnvalue "/Script/AIModule.AISense_Sight")
    (return "NewEnumerator0")
    (elif (== _returnvalue "/Script/AIModule.AISense_Hearing")
      (return "NewEnumerator1")
      (else
        (return "NewEnumerator2")))))

(fn `HandleHearSense`
  (params (Actor :type "Actor Object Reference") (Stimulus :type "AIStimulus Structure"))
  (bind _returnvalue (`AIPerceptionSystem.GetSenseClassForStimulus` Stimulus))
  (if (not (== _returnvalue "/Script/AIModule.AISenseConfig_Hearing"))
    (return)))

(fn `RobotSoundEvent`
  (params (AkEvent :type "AkAudioEvent Object Reference") (StateTag :type "GameplayTag Structure") (GenerateShock :type Boolean) (ShockGenerated :type "Float (double-precision)") (SenseType :type "/Game/Blueprints/Enumerators/E_SenseType Enum" :default "NewEnumerator1"))
  (`StateTreeComponent.SendStateTreeEvent` (`self.StateTreeAI`) (make `StateTreeEvent` StateTag))
  (`AkGameplayStatics.PostEvent` AkEvent (`self.K2_GetPawn`))
  (if GenerateShock
    (`self.GenerateShock` ShockGenerated SenseType)
    (return)
    (else
      (return))))

(fn `SetNavBlockArea`
  (params (NavArea :type "NavArea Class Reference"))
  (for _array_element (`self.NavBlocks`)
    (`NavModifierComponent.SetAreaClass` (`/Game/Blueprints/AI/Navigation/BP_NavBlock.NavModifier` _array_element) NavArea)))

(fn `UserConstructionScript`)