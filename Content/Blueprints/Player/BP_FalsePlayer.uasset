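; BP_FalsePlayer is a stand-in player body that plays the visual transition when possessing or leaving possession.
; PossessingAnimation stores a duration and endpoints, sets the rotation, picks shrink or grow scaling from the Possessing flag and unhides the actor.
; Tick counts the timer down, lerping the capsule's location and the skeletal mesh's scale, then hides the actor once the timer runs out.
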(event `self.ReceiveTick`
  (params (DeltaSeconds :type "Float (single-precision)"))
  (if (> (`self.Timer`) 0.0)
    (bind _output_get (set `self.Timer` (- (`self.Timer`) DeltaSeconds)))
    (`|ExecutionSequence`
      (:`then_0`
        (bind _returnvalue (`KismetMathLibrary.SafeDivide` _output_get (`self.AnimTime`)))
        (`SceneComponent.K2_SetWorldLocation` (`self.Capsule`) (`KismetMathLibrary.VLerp` (`self.EndLocation`) (`self.StartLocation`) _returnvalue) false false))
      (:`then_1`
        (`SceneComponent.SetRelativeScale3D` (`self.SkeletalMesh`) (`KismetMathLibrary.Conv_DoubleToVector` (`KismetMathLibrary.Lerp` (`self.EndScale`) (`self.StartScale`) _returnvalue)))))
    (else
      (`self.SetActorHiddenInGame` true))))

(event `PossessingAnimation`
  (params (Possessing :type Boolean) (Time :type "Float (double-precision)") (Start :type "Vector Structure") (End :type "Vector Structure") (Rotation :type "Rotator Structure"))
  (bind _output_get (set `self.AnimTime` Time))
  (set `self.Timer` _output_get)
  (set `self.StartLocation` Start)
  (set `self.EndLocation` End)
  (if Possessing
    (set `self.StartScale` 1.0)
    (set `self.EndScale` 0.0)
    (else
      (set `self.StartScale` 0.0)
      (set `self.EndScale` 1.0)))
  (`self.SetActorHiddenInGame` false)
  (`self.K2_SetActorRotation` Rotation true))

(fn `UserConstructionScript`)