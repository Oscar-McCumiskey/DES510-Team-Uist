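; BP_AudioPulse is a short-lived visual pulse actor, filed under possessable interactables.
; On BeginPlay it creates a dynamic instance of M_AudioPulse on the Pulse component and plays the Scale timeline.
; The timeline drives the component's uniform world scale and the material's Opacity parameter together, then the actor destroys itself after a brief delay.
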(event `self.ReceiveBeginPlay`
  (bind _returnvalue (`PrimitiveComponent.CreateDynamicMaterialInstance` (`self.Pulse`) 0 "/Game/Art_Assets/Materials/M_AudioPulse.M_AudioPulse" "None"))
  (set `self.DynamicMaterial` _returnvalue)
  (bind (_direction _scale _opacity) (`Timeline|Scale` :!via `PlayFromStart`)
    (:`Update`
      (`SceneComponent.SetWorldScale3D` (`self.Pulse`) (`KismetMathLibrary.Conv_DoubleToVector` _scale))
      (`MaterialInstanceDynamic.SetScalarParameterValue` (`self.DynamicMaterial`) "Opacity" _opacity))
    (:`Finished`
      (`KismetSystemLibrary.Delay` 0.2)
      (`self.K2_DestroyActor`))))

(fn `UserConstructionScript`)