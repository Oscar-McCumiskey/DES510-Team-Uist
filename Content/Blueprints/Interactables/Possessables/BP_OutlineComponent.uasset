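; Outline component for possessable appliances that colours the mesh to show neutral, selected or possessed state.
; On BeginPlay it applies a dynamic instance of the outline material as the static mesh overlay, raising an error if none is set.
; State events set its Colour parameter through SetColourByType.
; Selection uses a short retriggerable delay, so the outline returns to neutral once calls stop, unless flagged possessed.
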(event `self.ReceiveBeginPlay`
  (bind _outlinematerial (`self.OutlineMaterial`))
  (`/Engine/EditorBlueprintResources/StandardMacros.IsValid` _outlinematerial
    (:`Is Valid`
      (bind _returnvalue (`KismetMaterialLibrary.CreateDynamicMaterialInstance` _outlinematerial))
      (bind _output_get (set `self.DynamicMaterial` _returnvalue))
      (bind _aspossessable_appliance (cast `PossessableAppliance` (`self.GetOwner`)))
      (`MeshComponent.SetOverlayMaterial` (`PossessableAppliance.StaticMesh` _aspossessable_appliance) _output_get)
      (`MaterialInstanceDynamic.SetVectorParameterValue` (`self.DynamicMaterial`) "Colour" (`self.NeutralColour`)))
    (:`Is Not Valid`
      (`KismetSystemLibrary.RaiseScriptError` "Object has no outline material"))))

(event `PossessedOutline`
  (`KismetSystemLibrary.DelayUntilNextTick`)
  (`self.SetColourByType` "NewEnumerator0")
  (`KismetSystemLibrary.PrintString` "Possessed"))

(event `NeutralOutline`
  (`self.SetColourByType` "NewEnumerator2")
  (`KismetSystemLibrary.PrintString` "Neutral"))

(event `SelectedOutline`
  (params (IsPossessed :type Boolean))
  (`self.SetColourByType` "NewEnumerator1")
  (`KismetSystemLibrary.RetriggerableDelay` 0.05)
  (if (not IsPossessed)
    (`self.SetColourByType` "NewEnumerator2")
    (`KismetSystemLibrary.PrintString` "Neutral")))

(fn `SetColourByType`
  (params (ColourType :type "/Game/Blueprints/Enumerators/E_OutlineColour Enum" :default "NewEnumerator0"))
  (locals (MaterialColour :type "LinearColor Structure"))
  (switch `/Game/Blueprints/Enumerators/E_OutlineColour` ColourType
    (:`NewEnumerator0`
      (set `local.MaterialColour` (`self.PossessedColour`)))
    (:`NewEnumerator1`
      (set `local.MaterialColour` (`self.SelectedColour`)))
    (:`NewEnumerator2`
      (set `local.MaterialColour` (`self.NeutralColour`))))
  (`MaterialInstanceDynamic.SetVectorParameterValue` (`self.DynamicMaterial`) "Colour" (`local.MaterialColour`)))