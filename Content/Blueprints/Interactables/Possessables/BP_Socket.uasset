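; BP_Socket is a possessable interactable that lets the player hop between the sockets listed on their BP_ThirdPersonCharacter.
; Abilities one and two step that character's CurrentSocket index forward or back with wraparound, hand Possessor to the chosen socket, and have the player controller possess it.
; Interact teleports a valid Possessor to just behind the socket's camera boom, matching the socket's rotation.
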(event `self.DoAbilityOneBlueprint`
  ; Cycle Sockets
  (bind _asbp_third_person_character (cast `/Game/ThirdPerson/Blueprints/BP_ThirdPersonCharacter` (`self.Possessor`)))
  (bind _sockets (`/Game/ThirdPerson/Blueprints/BP_ThirdPersonCharacter.Sockets` _asbp_third_person_character))
  (bind _output_get (set `/Game/ThirdPerson/Blueprints/BP_ThirdPersonCharacter.CurrentSocket` (`KismetMathLibrary.Wrap` (+ (`/Game/ThirdPerson/Blueprints/BP_ThirdPersonCharacter.CurrentSocket` _asbp_third_person_character) 1) -1 (- (`KismetArrayLibrary.Array_Length` _sockets) 1)) _asbp_third_person_character))
  (bind _output (`|GetArrayItem` _sockets _output_get))
  (set `PossessableAppliance.Possessor` (`self.Possessor`) _output)
  (bind _asbp_third_person_player_controller (cast `/Game/ThirdPerson/Blueprints/BP_ThirdPersonPlayerController` (`self.GetController`)))
  (`DES510_Team_UistPlayerController.PossessPawn` _asbp_third_person_player_controller _output))

(event `self.DoAbilityTwoBlueprint`
  ; Cycle Sockets
  (bind _asbp_third_person_character (cast `/Game/ThirdPerson/Blueprints/BP_ThirdPersonCharacter` (`self.Possessor`)))
  (bind _sockets (`/Game/ThirdPerson/Blueprints/BP_ThirdPersonCharacter.Sockets` _asbp_third_person_character))
  (bind _output_get (set `/Game/ThirdPerson/Blueprints/BP_ThirdPersonCharacter.CurrentSocket` (`KismetMathLibrary.Wrap` (+ (`/Game/ThirdPerson/Blueprints/BP_ThirdPersonCharacter.CurrentSocket` _asbp_third_person_character) -1) 0 (`KismetArrayLibrary.Array_Length` _sockets)) _asbp_third_person_character))
  (bind _output (`|GetArrayItem` _sockets _output_get))
  (set `PossessableAppliance.Possessor` (`self.Possessor`) _output)
  (bind _asbp_third_person_player_controller (cast `/Game/ThirdPerson/Blueprints/BP_ThirdPersonPlayerController` (`self.GetController`)))
  (`DES510_Team_UistPlayerController.PossessPawn` _asbp_third_person_player_controller _output))

(event `self.DoInteractBlueprint`
  (bind _possessor (`self.Possessor`))
  (bind _cameraboom (`self.CameraBoom`))
  (`/Engine/EditorBlueprintResources/StandardMacros.IsValid` _possessor
    (:`Is Valid`
      (`self.K2_SetActorLocationAndRotation` _possessor (+ (`SceneComponent.K2_GetComponentLocation` _cameraboom) (* (`SceneComponent.GetForwardVector` _cameraboom) -50.0)) (`self.K2_GetActorRotation`) false true))))

(fn `UserConstructionScript`)