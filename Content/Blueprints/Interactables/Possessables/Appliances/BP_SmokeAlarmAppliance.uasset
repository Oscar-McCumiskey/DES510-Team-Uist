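; Possessable smoke alarm appliance whose two abilities distract others with sound and light.
; Ability one plays a short beep, reports an "AlertAudio" noise and flashes the point light once via a timeline.
; Ability two reports "PanicAudio", then re-triggers a beep and flash timeline on Finished until FlashCount reaches FlashAmount, leaving a debug print each cycle.
; Possession and key presses fire Wwise events.
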(event `self.DoAbilityOneBlueprint`
  (`AkGameplayStatics.PostEvent` "/Game/WwiseAudio/Events/Default_Work_Unit/AkEvent_PlayerPossessionKeyPressed.AkEvent_PlayerPossessionKeyPressed")
  (`AkGameplayStatics.PostEvent` "/Game/WwiseAudio/Events/Default_Work_Unit/AkEvent_SmokeDetectorBeeps/AkEvent_SmokeDetectorShortBeep.AkEvent_SmokeDetectorShortBeep" self)
  (`AISense_Hearing.ReportNoiseEvent` (`self.K2_GetActorLocation`) 1.0 (`self.GetController`) 1000.0 "AlertAudio")
  (bind (_direction _intensity) (`Timeline|Flash Light` :!via `PlayFromStart`)
    (:`Update`
      (`LightComponent.SetIntensity` (`self.PointLight`) (* _intensity 100.0)))))

(event `self.ReceivePossessed`
  (params (NewController :type "Controller Object Reference"))
  (`AkGameplayStatics.PostEvent` "/Game/WwiseAudio/Events/Default_Work_Unit/AkEvent_PlayerPossession.AkEvent_PlayerPossession" self))

(event `self.DoAbilityTwoBlueprint`
  (`AkGameplayStatics.PostEvent` "/Game/WwiseAudio/Events/Default_Work_Unit/AkEvent_PlayerPossessionKeyPressed.AkEvent_PlayerPossessionKeyPressed")
  (`AISense_Hearing.ReportNoiseEvent` (`self.K2_GetActorLocation`) 1.0 (`self.GetController`) 1000.0 "PanicAudio")
  (if (< (`self.FlashCount`) (`self.FlashAmount`)) :!label _label
    (`AkGameplayStatics.PostEvent` "/Game/WwiseAudio/Events/Default_Work_Unit/AkEvent_SmokeDetectorBeeps/AkEvent_SmokeDetectorSingleBeep.AkEvent_SmokeDetectorSingleBeep" self)
    (bind (_direction _intensity) (`Timeline|Flashing Light` :!via `PlayFromStart`)
      (:`Update`
        (`LightComponent.SetIntensity` (`self.PointLight`) (* _intensity 100.0)))
      (:`Finished`
        (`/Engine/EditorBlueprintResources/StandardMacros.IncrementInt` (`self.FlashCount`)
          (:`  `
            (`KismetSystemLibrary.PrintString` "Hello")
            (goto _label)))))
    (else
      (set `self.FlashCount` 0))))

(fn `UserConstructionScript`)