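; BP_SmartHomeAppliance is a possessable smart home voice assistant that the player uses to make noise that AI can hear.
; Possession posts a Wwise sound event, and both abilities post key-press and assistant voice-line events.
; Each ability also reports an AI noise event at the appliance with the same range, tagged as alert audio for the first and spooked audio for the second.
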(event `self.ReceivePossessed`
  (params (NewController :type "Controller Object Reference"))
  (`AkGameplayStatics.PostEvent` "/Game/WwiseAudio/Events/Default_Work_Unit/AkEvent_PlayerPossession.AkEvent_PlayerPossession" self))

(event `self.ReceiveUnpossessed`
  (params (OldController :type "Controller Object Reference")))

(event `self.DoAbilityOneBlueprint`
  (`AkGameplayStatics.PostEvent` "/Game/WwiseAudio/Events/Default_Work_Unit/AkEvent_PlayerPossessionKeyPressed.AkEvent_PlayerPossessionKeyPressed" self)
  (`AkGameplayStatics.PostEvent` "/Game/WwiseAudio/Events/Default_Work_Unit/AkEvent_AlexaAssistantVoiceLines.AkEvent_AlexaAssistantVoiceLines" self)
  (`AISense_Hearing.ReportNoiseEvent` (`self.K2_GetActorLocation`) 1.0 (`self.GetController`) 1000.0 "AlertAudio"))

(event `self.DoAbilityTwoBlueprint`
  (`AkGameplayStatics.PostEvent` "/Game/WwiseAudio/Events/Default_Work_Unit/AkEvent_PlayerPossessionKeyPressed.AkEvent_PlayerPossessionKeyPressed" self)
  (`AkGameplayStatics.PostEvent` "/Game/WwiseAudio/Events/Default_Work_Unit/AkEvent_AlexaAssistantVoiceLines.AkEvent_AlexaAssistantVoiceLines" self)
  (`AISense_Hearing.ReportNoiseEvent` (`self.K2_GetActorLocation`) 1.0 (`self.GetController`) 1000.0 "SpookedAudio"))

(fn `UserConstructionScript`)