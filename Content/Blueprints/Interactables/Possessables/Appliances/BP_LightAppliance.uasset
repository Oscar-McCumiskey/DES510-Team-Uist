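; BP_LightAppliance is a possessable ceiling light whose abilities flicker it or cycle its colour.
; On BeginPlay it creates a dynamic emissive material, and each ability drives that material and the light component together through a timeline.
; Both abilities report an "AlertVisual" noise event to AI perception.
; Wwise events play on possession and flicker, with the flicker sound repeated by a timer.
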(event `self.ReceiveBeginPlay`
  (bind _returnvalue (`PrimitiveComponent.CreateDynamicMaterialInstance` (`self.StaticMesh`) 1 "/Game/Art_Assets/Models/Ceiling_Light/Materials/Hanging_Ceiling_Lights1.Hanging_Ceiling_Lights1" "None"))
  (bind _output_get (set `self.DynamicEmissiveMaterial` _returnvalue))
  (`MaterialInstanceDynamic.SetScalarParameterValue` _output_get "EmissiveColorMapWeight" 1.0)
  (`MaterialInstanceDynamic.SetVectorParameterValue` _output_get "LightColour" (struct :`R` 1.0 :`G` 1.0 :`B` 1.0 :`A` 1.0)))

(event `self.ReceivePossessed`
  (params (NewController :type "Controller Object Reference"))
  (`KismetSystemLibrary.DelayUntilNextTick`)
  (`AkGameplayStatics.PostEvent` "/Game/WwiseAudio/Events/Default_Work_Unit/AkEvent_PlayerPossession.AkEvent_PlayerPossession" self))

(event `self.DoAbilityOneBlueprint`
  (`AkGameplayStatics.PostEvent` "/Game/WwiseAudio/Events/Default_Work_Unit/AkEvent_LightFlicker.AkEvent_LightFlicker" self)
  (`AISense_Hearing.ReportNoiseEvent` (`self.K2_GetActorLocation`) 1.0 (`self.GetController`) 1000.0 "AlertVisual")
  (`KismetSystemLibrary.K2_SetTimerDelegate` (delegate `PlayFlickerSound`) 2.6)
  (bind (_direction _material_intensity _light_intensity) (`Timeline|Light Flicker` :!via `PlayFromStart`)
    (:`Update`
      (`MaterialInstanceDynamic.SetScalarParameterValue` (`self.DynamicEmissiveMaterial`) "EmissiveColorMapWeight" _material_intensity)
      (`LightComponent.SetIntensity` (`self.LightComponent`) (* _light_intensity 8.0)))))

(event `PlayFlickerSound`
  (`AkGameplayStatics.PostEvent` "/Game/WwiseAudio/Events/Default_Work_Unit/AkEvent_LightFlicker.AkEvent_LightFlicker" self))

(event `self.DoAbilityTwoBlueprint`
  (`AISense_Hearing.ReportNoiseEvent` (`self.K2_GetActorLocation`) 1.0 (`self.GetController`) 1000.0 "AlertVisual")
  (bind (_direction _ravemode) (`Timeline|Timeline` :!via `PlayFromStart`)
    (:`Update`
      (`MaterialInstanceDynamic.SetVectorParameterValue` (`self.DynamicEmissiveMaterial`) "LightColour" _ravemode)
      (`LightComponent.SetLightColor` (`self.LightComponent`) _ravemode true))))

(event `self.DoInteractBlueprint`)

(fn `UserConstructionScript`)