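; BP_Roomba is a possessable Roomba appliance that the player can inhabit and use to make noise.
; Its ability input plays a taunt sound and reports a noise event at its location for AI hearing.
; Possession plays a Wwise possession sound, and unpossession teleports a valid Possessor just above the Roomba, matching its rotation.
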(event `EnhancedInput|/Game/Input/Actions/IA_Ability1`
  (params (ActionValue :type Boolean) (ElapsedSeconds :type "Float (double-precision)") (TriggeredSeconds :type "Float (double-precision)") (InputAction :type "InputAction Object Reference" :default "/Game/Input/Actions/IA_Ability1.IA_Ability1"))
  (:`Triggered`
    (`AkGameplayStatics.PostEvent` "/Game/WwiseAudio/Events/Default_Work_Unit/AkEvent_RoombaTaunt.AkEvent_RoombaTaunt" self)
    (`AISense_Hearing.ReportNoiseEvent` (`self.K2_GetActorLocation`) 1.0 (`self.GetController`) 1000.0)
    (`KismetSystemLibrary.PrintString` "Sound")))

(event `self.ReceivePossessed`
  (params (NewController :type "Controller Object Reference"))
  (`AkGameplayStatics.PostEvent` "/Game/WwiseAudio/Events/Default_Work_Unit/AkEvent_PlayerPossession.AkEvent_PlayerPossession" self))

(event `self.ReceiveUnpossessed`
  (params (OldController :type "Controller Object Reference"))
  (bind _possessor (`self.Possessor`))
  (`/Engine/EditorBlueprintResources/StandardMacros.IsValid` _possessor
    (:`Is Valid`
      (`self.K2_SetActorLocationAndRotation` _possessor (+ (`self.K2_GetActorLocation`) (0.0 0.0 50.0)) (`self.K2_GetActorRotation`) false true))))

(fn `UserConstructionScript`)