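; Possessable TV appliance whose two abilities make AI noise events tagged to alert or spook.
; Ability one plays static audio while a replayed timeline's event track steps the screen through an array of static materials, then restores the screen and plays shutdown audio.
; Ability two drives a dynamic material parameter from the Handprints timeline's opacity curve, then restores the default screen material.
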(event `self.ReceiveBeginPlay`
  (bind _returnvalue (`PrimitiveComponent.CreateDynamicMaterialInstance` (`self.StaticMesh`) 1 "/Game/Art_Assets/Models/TV/Materials/TV1_004.TV1_004" "None"))
  (bind _output_get (set `self.DynamicMaterial` _returnvalue))
  (`MaterialInstanceDynamic.SetScalarParameterValue` _output_get "DiffuseColorMapWeight" 0.0)
  (`PrimitiveComponent.SetMaterial` (`self.StaticMesh`) 1 "/Game/Art_Assets/Models/TV/Materials/TV1.TV1"))

(event `self.ReceiveTick`
  (params (DeltaSeconds :type "Float (single-precision)")))

(event `self.ReceivePossessed`
  (params (NewController :type "Controller Object Reference"))
  (`AkGameplayStatics.PostEvent` "/Game/WwiseAudio/Events/Default_Work_Unit/AkEvent_PlayerPossession.AkEvent_PlayerPossession" self))

(event `self.ReceiveUnpossessed`
  (params (OldController :type "Controller Object Reference")))

(event `self.DoAbilityOneBlueprint`
  (`AkGameplayStatics.PostEvent` "/Game/WwiseAudio/Events/Default_Work_Unit/AkEvent_PlayerPossessionKeyPressed.AkEvent_PlayerPossessionKeyPressed" self)
  (`AkGameplayStatics.PostEvent` "/Game/WwiseAudio/Events/Default_Work_Unit/AkEvent_TelevisionStatic.AkEvent_TelevisionStatic" self)
  (`AISense_Hearing.ReportNoiseEvent` (`self.K2_GetActorLocation`) 1.0 (`self.GetController`) 1000.0 "AlertVisual")
  (set `self.LoopCount` 0)
  (set `self.Count` 0 :!label _label)
  (`Timeline|Static` :!via `PlayFromStart`
    (:`Finished`
      (if (>= (`self.LoopCount`) 5)
        (`PrimitiveComponent.SetMaterial` (`self.StaticMesh`) 1 "/Game/Art_Assets/Models/TV/Materials/TV1.TV1")
        (`AkGameplayStatics.PostAndWaitForEndOfEvent` "/Game/WwiseAudio/Events/Default_Work_Unit/STOP_EVENTS/AkEvent_STOP_TelevisionStatic.AkEvent_STOP_TelevisionStatic" self)
        (`AkGameplayStatics.PostEvent` "/Game/WwiseAudio/Events/Default_Work_Unit/AkEvent_TVShutDown.AkEvent_TVShutDown" self)
        (else
          (`/Engine/EditorBlueprintResources/StandardMacros.IncrementInt` (`self.LoopCount`)
            (:`  `
              (goto _label))))))
    (:`Static`
      (`PrimitiveComponent.SetMaterial` (`self.StaticMesh`) 1 (`|GetArrayItem` (`self.StaticMaterials`) (`self.Count`)))
      (`/Engine/EditorBlueprintResources/StandardMacros.IncrementInt` (`self.Count`)))))

(event `self.DoAbilityTwoBlueprint`
  (bind _dynamicmaterial (`self.DynamicMaterial`))
  (`AISense_Hearing.ReportNoiseEvent` (`self.K2_GetActorLocation`) 1.0 (`self.GetController`) 1000.0 "SpookedVisual")
  (`PrimitiveComponent.SetMaterial` (`self.StaticMesh`) 1 _dynamicmaterial)
  (`MaterialInstanceDynamic.SetScalarParameterValue` _dynamicmaterial "DiffuseColorMapWeight" 0.0)
  (bind (_direction _opacity) (`Timeline|Handprints` :!via `PlayFromStart`)
    (:`Update`
      (`MaterialInstanceDynamic.SetScalarParameterValue` (`self.DynamicMaterial`) "DiffuseColorMapWeight" (`.A` (break `LinearColor` _opacity))))
    (:`Finished`
      (`PrimitiveComponent.SetMaterial` (`self.StaticMesh`) 1 "/Game/Art_Assets/Models/TV/Materials/TV1.TV1"))))

(fn `UserConstructionScript`)