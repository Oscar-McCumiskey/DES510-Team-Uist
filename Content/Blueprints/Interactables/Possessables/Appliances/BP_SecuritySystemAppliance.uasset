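; A possessable security system appliance that gives the possessing player a burglar alarm and level-wide door control.
; On BeginPlay it caches every BP_Door flagged Unlockable.
; Ability one plays the alarm, reports a "PanicAudio" noise event for AI and spawns an audio pulse at its location.
; Ability two closes all cached doors, passing a lock time; the "Search" noise logic is left unconnected.
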(event `self.ReceiveBeginPlay`
  (bind _outactors (`GameplayStatics.GetAllActorsOfClass` "/Game/Blueprints/Interactables/BP_Door.BP_Door_C"))
  (for _array_element _outactors
    (if (`/Game/Blueprints/Interactables/BP_Door.Unlockable` _array_element)
      (`KismetArrayLibrary.Array_Add` (`self.Doors`) _array_element))))

(event `self.ReceivePossessed`
  (params (NewController :type "Controller Object Reference")))

(event `self.DoAbilityOneBlueprint`
  (`AkGameplayStatics.PostEvent` "/Game/WwiseAudio/Events/Default_Work_Unit/AkEvent_PlayerPossessionKeyPressed.AkEvent_PlayerPossessionKeyPressed")
  (`AkGameplayStatics.PostEvent` "/Game/WwiseAudio/Events/Default_Work_Unit/AkEvent_BurglarAlarm.AkEvent_BurglarAlarm" self)
  (`AISense_Hearing.ReportNoiseEvent` (`self.K2_GetActorLocation`) 1.0 (`self.GetController`) 1000.0 "PanicAudio")
  (`|SpawnActorFromClass` "/Game/Blueprints/Interactables/Possessables/BP_AudioPulse.BP_AudioPulse_C" (`KismetMathLibrary.MakeTransform` (`self.K2_GetActorLocation`)) "AlwaysSpawn" "MultiplyWithRoot" null null))

(event `self.DoAbilityTwoBlueprint`
  (for _array_element (`self.Doors`)
    (`/Game/Blueprints/Interactables/BP_Door.CloseDoor` _array_element (`self.DoorLockTime`))))

(fn `UserConstructionScript`)