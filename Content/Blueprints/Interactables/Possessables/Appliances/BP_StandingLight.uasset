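; Possessable standing light that gives its possessor two abilities, each reporting an "AlertVisual" noise event to draw AI attention.
; BeginPlay creates a dynamic emissive material on the mesh so timelines can drive it alongside the point light.
; Ability one flickers emissive weight and light intensity, playing a Wwise flicker sound immediately and again on a timer.
; Ability two runs a RaveMode timeline that animates the colour of both material and light.
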(event `self.ReceiveBeginPlay`
  (bind _returnvalue (`PrimitiveComponent.CreateDynamicMaterialInstance` (`self.StaticMesh`) 2 "/Game/Art_Assets/Models/Ceiling_Light/Materials/Hanging_Ceiling_Lights1.Hanging_Ceiling_Lights1" "None"))
  (bind _output_get (set `self.DynamicEmissiveMaterial` _returnvalue))
  (`MaterialInstanceDynamic.SetScalarParameterValue` _output_get "EmissiveColorMapWeight" 1.0))

(event `self.ReceivePossessed`
  (params (NewController :type "Controller Object Reference")))

(event `self.DoAbilityOneBlueprint`
  (`AkGameplayStatics.PostEvent` "/Game/WwiseAudio/Events/Default_Work_Unit/AkEvent_LightFlicker.AkEvent_LightFlicker" self)
  (`AISense_Hearing.ReportNoiseEvent` (`self.K2_GetActorLocation`) 1.0 (`self.GetController`) 1000.0 "AlertVisual")
  (`KismetSystemLibrary.K2_SetTimerDelegate` (delegate `PlayFlickerSound`) 2.6)
  (bind (_direction _material_intensity _light_intensity) (`Timeline|Timeline` :!via `PlayFromStart`)
    (:`Update`
      (`MaterialInstanceDynamic.SetScalarParameterValue` (`self.DynamicEmissiveMaterial`) "EmissiveColorMapWeight" _material_intensity)
      (`LightComponent.SetIntensity` (`self.PointLight`) (* _light_intensity 8.0)))))

(event `PlayFlickerSound`
  (`AkGameplayStatics.PostEvent` "/Game/WwiseAudio/Events/Default_Work_Unit/AkEvent_LightFlicker.AkEvent_LightFlicker" self))

(event `self.DoAbilityTwoBlueprint`
  (`AISense_Hearing.ReportNoiseEvent` (`self.K2_GetActorLocation`) 1.0 (`self.GetController`) 1000.0 "AlertVisual")
  (bind (_direction _ravemode) (`Timeline|RaveMode` :!via `PlayFromStart`)
    (:`Update`
      (`MaterialInstanceDynamic.SetVectorParameterValue` (`self.DynamicEmissiveMaterial`) "LightColour" _ravemode)
      (`LightComponent.SetLightColor` (`self.PointLight`) _ravemode true))))

(fn `UserConstructionScript`)