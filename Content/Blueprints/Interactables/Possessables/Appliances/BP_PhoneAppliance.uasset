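; BP_PhoneAppliance is a possessable phone interactable that lets the player send text messages.
; A sphere overlap shows its widget while BP_ThirdPersonCharacter is nearby.
; On possession it takes the inbox widget from the player controller's HUD and shows it, hiding it again on unpossession.
; Its two ability events send player texts through that inbox, distinguished by ability index.
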(event `self.ReceiveBeginPlay`
  (`SceneComponent.SetVisibility` (`self.Widget`) false false))

(event `self.Sphere.OnComponentBeginOverlap`
  (params (OverlappedComponent :type "PrimitiveComponent Object Reference") (OtherActor :type "Actor Object Reference") (OtherComp :type "PrimitiveComponent Object Reference") (OtherBodyIndex :type Integer) (bFromSweep :type Boolean) (SweepResult :type "HitResult Structure (by ref)"))
  (if (== (`GameplayStatics.GetObjectClass` OtherActor) "/Game/ThirdPerson/Blueprints/BP_ThirdPersonCharacter.BP_ThirdPersonCharacter_C")
    (`SceneComponent.SetVisibility` (`self.Widget`) true false)))

(event `self.Sphere.OnComponentEndOverlap`
  (params (OverlappedComponent :type "PrimitiveComponent Object Reference") (OtherActor :type "Actor Object Reference") (OtherComp :type "PrimitiveComponent Object Reference") (OtherBodyIndex :type Integer))
  (if (== (`GameplayStatics.GetObjectClass` OtherActor) "/Game/ThirdPerson/Blueprints/BP_ThirdPersonCharacter.BP_ThirdPersonCharacter_C")
    (`SceneComponent.SetVisibility` (`self.Widget`) false false)))

(event `self.ReceivePossessed`
  (params (NewController :type "Controller Object Reference"))
  (bind _asbp_third_person_player_controller (cast `/Game/ThirdPerson/Blueprints/BP_ThirdPersonPlayerController` NewController))
  (bind _output_get (set `self.PlayerController` _asbp_third_person_player_controller))
  (bind _output_get_2 (set `self.PhoneInbox` (`/Game/Blueprints/UI/W_PlayerHUD.W_PhoneInbox` (`/Game/Blueprints/UI/PlayerHUD.HUD` (`/Game/ThirdPerson/Blueprints/BP_ThirdPersonPlayerController.PlayerHUD` _output_get)))))
  (`Widget.SetVisibility` _output_get_2 "HitTestInvisible"))

(event `self.ReceiveUnpossessed`
  (params (OldController :type "Controller Object Reference"))
  (`Widget.SetVisibility` (`self.PhoneInbox`) "Hidden"))

(event `self.DoAbilityOneBlueprint`
  (`/Game/Blueprints/UI/Phone/W_PhoneInbox.SendTextMessage` (`self.PhoneInbox`) true 0))

(event `self.DoAbilityTwoBlueprint`
  (`/Game/Blueprints/UI/Phone/W_PhoneInbox.SendTextMessage` (`self.PhoneInbox`) true 1))

(fn `UserConstructionScript`)