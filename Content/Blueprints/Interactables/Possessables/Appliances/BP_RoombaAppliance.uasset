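; Possessable Roomba appliance that the player can take over and drive, with an AI controller running it otherwise.
; Possession swaps movement speed; on player release it teleports the possessor just above the Roomba and hands control back to the cached AI controller.
; Move input drives Wwise motor audio from start through loop to end.
; Ability one plays a taunt and reports an "Alert" noise for AI hearing; ability two is empty.
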(event `self.ReceivePossessed`
  (params (NewController :type "Controller Object Reference"))
  ; Possession Logic
  (if (`self.IsPossessedByPlayer` NewController)
    (`AkGameplayStatics.PostEvent` "/Game/WwiseAudio/Events/Default_Work_Unit/AkEvent_PlayerPossession.AkEvent_PlayerPossession" self)
    (set `FloatingPawnMovement.MaxSpeed` (`self.PossessedSpeed`) (`self.MovementComponent`))
    (else
      (set `self.AIController` NewController))))

(event `self.ReceiveUnpossessed`
  (params (OldController :type "Controller Object Reference"))
  (bind _possessor (`self.Possessor`))
  (bind _aicontroller (`self.AIController`))
  ; Possession Logic
  (if (`self.IsPossessedByPlayer` OldController)
    (set `FloatingPawnMovement.MaxSpeed` (`self.UnpossessedSpeed`) (`self.MovementComponent`))
    (`/Engine/EditorBlueprintResources/StandardMacros.IsValid` _possessor
      (:`Is Valid`
        (`self.K2_SetActorLocationAndRotation` _possessor (+ (`self.K2_GetActorLocation`) (0.0 0.0 50.0)) (`self.K2_GetActorRotation`) false true)
        (`/Engine/EditorBlueprintResources/StandardMacros.IsValid` _aicontroller
          (:`Is Valid`
            (`Controller.Possess` _aicontroller self)))))))

(event `EnhancedInput|/Game/Input/Actions/IA_Move`
  (params (ActionValue :type "Vector2D Structure") (ElapsedSeconds :type "Float (double-precision)") (TriggeredSeconds :type "Float (double-precision)") (InputAction :type "InputAction Object Reference" :default "/Game/Input/Actions/IA_Move.IA_Move"))
  ; Roomba Movement
  (:`Started`
    (bind _output_get (set `self.IsMoving` true))
    (`AkGameplayStatics.PostAndWaitForEndOfEvent` "/Game/WwiseAudio/Events/Default_Work_Unit/AkEvent_RoombaMovement/AkEvent_RoombaLoopSTART.AkEvent_RoombaLoopSTART" self)
    (if _output_get
      (`AkGameplayStatics.PostEvent` :`AkEvent` "/Game/WwiseAudio/Events/Default_Work_Unit/AkEvent_RoombaMovement/AkEvent_RoombaLoopMAIN.AkEvent_RoombaLoopMAIN" :`Actor` self :`bStopWhenAttachedToDestroyed` false)))
  (:`Completed`
    (set `self.IsMoving` false)
    (`AkGameplayStatics.PostEvent` "/Game/WwiseAudio/Events/Default_Work_Unit/AkEvent_STOP_RoombaLoopSTART.AkEvent_STOP_RoombaLoopSTART" self)
    (`AkGameplayStatics.PostEvent` "/Game/WwiseAudio/Events/Default_Work_Unit/AkEvent_STOP_RoombaLoopMAIN.AkEvent_STOP_RoombaLoopMAIN" self)
    (`AkGameplayStatics.PostEvent` "/Game/WwiseAudio/Events/Default_Work_Unit/AkEvent_RoombaMovement/AkEvent_RoombaLoopEND.AkEvent_RoombaLoopEND" self)))

(event `self.DoAbilityOneBlueprint`
  ; Ability Blueprint Logic
  (`AkGameplayStatics.PostEvent` "/Game/WwiseAudio/Events/Default_Work_Unit/AkEvent_RoombaTaunt.AkEvent_RoombaTaunt" self)
  (`AISense_Hearing.ReportNoiseEvent` (`self.K2_GetActorLocation`) 1.0 (`self.GetController`) 1000.0 "Alert"))

(event `self.DoAbilityTwoBlueprint`
  ; Ability Blueprint Logic
)

(fn `UserConstructionScript`)