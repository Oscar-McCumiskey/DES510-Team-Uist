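; BP_VinylAppliance is a possessable hi-fi vinyl player whose ability raises a "Panic" noise event and plays music.
; Possession posts a Wwise possession sound, while unpossession does nothing.
; Ability one reports the noise at the actor's location, waits for the key-press sound to end, then starts the activation and music events.
; After a Duration delay, it stops the music and plays a vinyl scratch.
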(event `self.ReceivePossessed`
  (params (NewController :type "Controller Object Reference"))
  (`AkGameplayStatics.PostEvent` "/Game/WwiseAudio/Events/Default_Work_Unit/AkEvent_PlayerPossession.AkEvent_PlayerPossession" self))

(event `self.ReceiveUnpossessed`
  (params (OldController :type "Controller Object Reference")))

(event `self.DoAbilityOneBlueprint`
  (`AISense_Hearing.ReportNoiseEvent` (`self.K2_GetActorLocation`) 1.0 (`self.GetController`) 1000.0 "Panic")
  (`AkGameplayStatics.PostAndWaitForEndOfEvent` "/Game/WwiseAudio/Events/Default_Work_Unit/AkEvent_PlayerPossessionKeyPressed.AkEvent_PlayerPossessionKeyPressed" self)
  (`AkGameplayStatics.PostEvent` "/Game/WwiseAudio/Events/Default_Work_Unit/AkEvent_HiFiStereoSystemActivate.AkEvent_HiFiStereoSystemActivate" self)
  (`AkGameplayStatics.PostEvent` "/Game/WwiseAudio/Events/Default_Work_Unit/AkEvent_HiFiStereoSystemMusic.AkEvent_HiFiStereoSystemMusic" self)
  (`KismetSystemLibrary.Delay` (`self.Duration`))
  (`AkGameplayStatics.PostEvent` "/Game/WwiseAudio/Events/Default_Work_Unit/STOP_EVENTS/AkEvent_STOP_HiFiStereoSystemMusic.AkEvent_STOP_HiFiStereoSystemMusic" self)
  (`AkGameplayStatics.PostEvent` "/Game/WwiseAudio/Events/Default_Work_Unit/AkEvent_HiFiStereoSystemVinylScratch.AkEvent_HiFiStereoSystemVinylScratch" self))

(fn `UserConstructionScript`)